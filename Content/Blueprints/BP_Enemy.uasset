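; Melee enemy character that chases BP_Player and fights with physics-driven sword swings and blocks.
; Physical animation partially ragdolls both arms, and forward forces swing the right arm on a looping timer or push out the left while randomly blocking.
; Sword collision is enabled briefly per swing and damages a non-blocking player on overlap.
; TakeDamage kills it outright, switching to full ragdoll and stopping movement, attacks and blocking.
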(event OnComponentBeginOverlap(Sword)
  (params (OverlappedComponent :type Primitive%20Component%20Object%20Reference) (OtherActor :type Actor%20Object%20Reference) (OtherComp :type Primitive%20Component%20Object%20Reference) (OtherBodyIndex :type Integer) (bFromSweep :type Boolean) (SweepResult :type Hit%20Result%20Structure%20%28by%20ref%29))
  ;[1 1 1] Sword Hit Detection
  (bind _asbp_player (Utilities|Casting|CastToBP_Player OtherActor))
  (if (Math|Boolean|ANDBoolean (Actor|ActorHasTag _asbp_player "Player") (Variables|Default|GetSwordUsed) (not (Variables|/Game/Blueprints/BP_Player.BP_Player_C|Getblocking _asbp_player)))
    (Audio|PlaySound2D 0 0.4 1.0 0.0 0 0)
    (Default|TakeDamage _asbp_player) ; BP_Player's Take Damage
  ))

(event EventBeginPlay
  ;[1 1 1] EventBeginPlay
  (CallFunction|ActiveRagdoll)
  (Utilities|Time|SetTimerbyFunctionName 0 "BlockTimer" (Variables|Default|GetBlockChangeTime) true)
  (Utilities|Time|SetTimerbyFunctionName 0 "Attack" 2.0 true))

(event EventTick
  (params (DeltaSeconds :type Float%20%28single-precision%29))
  ;[1 1 1] EventTick
  (if (not (Variables|Default|GetDead))
    (CallFunction|ChasePlayer)
    (if (Variables|Default|GetBlocking) ; Blocking state
      (Class|SkeletalMeshComponent|AddForcetoAllBodiesBelow (Variables|Character|GetMesh) (* (Transformation|GetActorForwardVector) "20000.000000,20000.000000,0.000000") (Variables|Default|GetLeftArmBone) false true))))

(fn ConstructionScript)

(fn ChasePlayer
  (bind _returnvalue (Actor|GetActorOfClass "/Game/Blueprints/BP_Player.BP_Player_C"))
  (AI|Navigation|MovetoLocation (AI|GetAIController self) (Transformation|GetActorLocation _returnvalue) 1e+02 true true false true 0))

(fn ActiveRagdoll
  (Class|PhysicalAnimationComponent|SetSkeletalMeshComponent (Variables|Default|GetPhysicalAnimation) (Variables|Character|GetMesh))
  (Class|PhysicalAnimationComponent|ApplyPhysicalAnimationSettingsBelow (Variables|Default|GetPhysicalAnimation) (Variables|Default|GetRightArmBone) (Utilities|Struct|MakePhysicalAnimationData true 3e+02 1e+01 1e+01 1e+01) true)
  (Class|SkeletalMeshComponent|SetAllBodiesBelowSimulatePhysics (Variables|Character|GetMesh) (Variables|Default|GetRightArmBone) true false)
  (Class|PhysicalAnimationComponent|ApplyPhysicalAnimationSettingsBelow (Variables|Default|GetPhysicalAnimation) (Variables|Default|GetLeftArmBone) (Utilities|Struct|MakePhysicalAnimationData true 1e+03 1e+02 1e+02 1e+02) true)
  (Class|SkeletalMeshComponent|SetAllBodiesBelowSimulatePhysics (Variables|Character|GetMesh) (Variables|Default|GetLeftArmBone) true false))

(fn BlockTimer
  (bind _output_get (Variables|Default|SetBlocking (Math|Random|RandomBool)))
  (if _output_get
    (Variables|Default|SetBlockChangeTime 0.8)
    (else
      (Variables|Default|SetBlockChangeTime 1.5))))

(fn Attack
  (Variables|Default|SetSwordused true)
  (Class|SkeletalMeshComponent|AddForcetoAllBodiesBelow (Variables|Character|GetMesh) (* (Transformation|GetActorForwardVector) "100000.000000,100000.000000,0.000000") (Variables|Default|GetRightArmBone) false true)
  (Collision|SetCollisionEnabled (Variables|Default|GetSword) "QueryAndPhysics")
  (Utilities|Time|SetTimerbyFunctionName 0 "ResetAttack" 0.2))

(fn ResetAttack
  (Variables|Default|SetSwordused false)
  (Collision|SetCollisionEnabled (Variables|Default|GetSword) "NoCollision"))

(fn TakeDamage
  (Collision|SetCollisionEnabled (Variables|Collision|GetCapsuleComponent) "NoCollision")
  (Class|PhysicalAnimationComponent|SetSkeletalMeshComponent (Variables|Default|GetPhysicalAnimation))
  (Physics|SetSimulatePhysics (Variables|Character|GetMesh) true) ; Ragdoll mode
  (Pawn|Components|CharacterMovement|DisableMovement (Variables|Character|GetCharacterMovement))
  (Variables|Default|SetDead true)
  (Class|KismetSystemLibrary|PauseTimer 0 "Attack")
  (Class|KismetSystemLibrary|PauseTimer 0 "BlockTimer")
  (Variables|Default|SetBlocking false)
  (Variables|Default|SetSwordUsed false))