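; BP_Player is the player character, with movement, look, sword, shield, a pause menu and a countdown that destroys it at zero.
; BeginPlay shows timer and controls widgets, while Tick uses a Delay to step minutes and seconds down.
; Hitbox overlaps with Enemy-tagged actors destroy the player unless blocking; sword hitbox overlaps destroy enemies during a brief swing window.
; An ActiveRagdoll physical-animation function exists but is never called.
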(event OnComponentBeginOverlap(Hitbox)
  (params (OverlappedComponent :type Primitive%20Component%20Object%20Reference) (OtherActor :type Actor%20Object%20Reference) (OtherComp :type Primitive%20Component%20Object%20Reference) (OtherBodyIndex :type Integer) (bFromSweep :type Boolean) (SweepResult :type Hit%20Result%20Structure%20%28by%20ref%29))
  ;[1 1 1] Death when not blocking
  (if (Actor|ActorHasTag OtherActor "Enemy")
    (if (not (Variables|Default|Getblocking))
      (Actor|DestroyActor))))

(event OnComponentBeginOverlap(Swordhitbox)
  (params (OverlappedComponent :type Primitive%20Component%20Object%20Reference) (OtherActor :type Actor%20Object%20Reference) (OtherComp :type Primitive%20Component%20Object%20Reference) (OtherBodyIndex :type Integer) (bFromSweep :type Boolean) (SweepResult :type Hit%20Result%20Structure%20%28by%20ref%29))
  ;[1 1 1] Sword attack
  (if (Actor|ActorHasTag OtherActor "Enemy")
    (if (Variables|Default|GetSwordused)
      (Actor|DestroyActor OtherActor))))

(event EventTick
  (params (DeltaSeconds :type Float%20%28single-precision%29))
  ;[1 1 1] Timer
  (Utilities|FlowControl|Delay 1.0)
  (if (== (Variables|Default|GetSeconds) 0)
    (if (== (Variables|Default|GetMinutes) 0)
      (Actor|DestroyActor)
      (else
        (Variables|Default|SetSeconds 59)
        (Variables|Default|SetMinutes (- (Variables|Default|GetMinutes) 1))))
    (else
      (Variables|Default|SetSeconds (- (Variables|Default|GetSeconds) 1)))))

(event EventBeginPlay
  ;[1 1 1] Timer
  (bind _returnvalue (UserInterface|CreateWidget "/Game/Widgets/W_Timer.W_Timer_C"))
  (UserInterface|Viewport|AddtoViewport _returnvalue 0)
  (bind _returnvalue_2 (UserInterface|CreateWidget "/Game/Widgets/W_Controls.W_Controls_C"))
  (UserInterface|Viewport|AddtoViewport _returnvalue_2 0))

(event Input|ActionEvents|InputActionShield
  (params (Key :type Key%20Structure :default "None"))
  ;[1 1 1] Shield
  (:Pressed
    (Variables|Default|Setblocking true)
    (Development|PrintString "Blocking"))
  (:Released
    (Variables|Default|Setblocking false)
    (Development|PrintString "Not blocking")))

(event Input|ActionEvents|InputActionSwordSwing
  (params (Key :type Key%20Structure :default "None"))
  ;[1 1 1] Sword swing
  (:Pressed
    (Variables|Default|SetSwordused true)
    (Utilities|FlowControl|Delay 0.25)
    (Variables|Default|SetSwordused false)
    (Development|PrintString "sword swung"))
  (:Released
    (Variables|Default|SetSwordused false)))

(event Input|ActionEvents|InputActionPause_Game
  (params (Key :type Key%20Structure :default "None"))
  ;[1 1 1] Pause
  (:Pressed
    (if (Variables|Default|GetIsPaused)
      (Widget|RemovefromParent (stale _returnvalue))
      (Game|SetGamePaused false)
      (Variables|Default|SetIsPaused false)
      (else
        (bind _returnvalue (UserInterface|CreateWidget "/Game/Widgets/W_PauseMenu.W_PauseMenu_C"))
        (UserInterface|Viewport|AddtoViewport _returnvalue 0)
        (Game|SetGamePaused true)
        (Variables|Default|SetIsPaused true)))))

(event Input|AxisEvents|InputAxisPlayer_Locomotion
  (params (AxisValue :type Float%20%28single-precision%29))
  ;[1 1 1] Player Movement
  (Pawn|Input|AddMovementInput (Transformation|GetActorForwardVector) (* AxisValue (Variables|Default|GetPlayer_Speed)) false))

(event Input|AxisEvents|InputAxisPlayer_Strafe
  (params (AxisValue :type Float%20%28single-precision%29))
  ;[1 1 1] Player Movement
  (Pawn|Input|AddMovementInput (Transformation|GetActorRightVector) AxisValue false))

(event Input|AxisEvents|InputAxisPlayer_HLook
  (params (AxisValue :type Float%20%28single-precision%29))
  ;[1 1 1] Look Controls
  (Pawn|Input|AddControllerYawInput AxisValue))

(event Input|AxisEvents|InputAxisPLayer_Vlook
  (params (AxisValue :type Float%20%28single-precision%29))
  ;[1 1 1] Look Controls
  (Pawn|Input|AddControllerPitchInput AxisValue))

(fn ConstructionScript)

(fn ActiveRagdoll
  (Class|PhysicalAnimationComponent|SetSkeletalMeshComponent (Variables|Default|GetPhysicalAnimation) (Variables|Character|GetMesh))
  (Class|PhysicalAnimationComponent|ApplyPhysicalAnimationSettingsBelow (Variables|Default|GetPhysicalAnimation) (Variables|Default|GetBoneName) (Utilities|Struct|MakePhysicalAnimationData true 4e+03 1e+02 1e+02 1e+02) true)
  (Class|SkeletalMeshComponent|SetAllBodiesBelowSimulatePhysics (Variables|Character|GetMesh) (Variables|Default|GetBoneName) true false)
  (Utilities|Time|SetTimerbyFunctionName 0 "RandomizeActions" 1.5 true)
  (Utilities|Time|SetTimerbyFunctionName 0 "Attack" 2.0 true))