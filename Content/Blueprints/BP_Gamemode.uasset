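; BP_Gamemode is a game mode Blueprint with logic for a pre-match freeze and for spawning enemies.
; WaitToPlay and MatchStart disable and restore walking movement on the Characters array.
; StartRound spawns one BP_Enemy at a random BP_EnemySpawnPoint.
; BeginPlay is empty, and the nodes that gather the player and enemies and start the MatchStart timer are disconnected.
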(event Custom|WaitToPlay
  (for _array_element (Variables|Default|GetCharacters)
    (bind _ascharacter (Utilities|Casting|CastToCharacter _array_element))
    (Pawn|Components|CharacterMovement|SetMovementMode (Variables|/Script/Engine.Character|GetCharacterMovement _ascharacter) "MOVE_None" 0)))

(event Custom|MatchStart
  (for _array_element (Variables|Default|GetCharacters)
    (bind _ascharacter (Utilities|Casting|CastToCharacter _array_element))
    (Pawn|Components|CharacterMovement|SetMovementMode (Variables|/Script/Engine.Character|GetCharacterMovement _ascharacter) "MOVE_Walking" 0)))

(event EventBeginPlay)

(fn ConstructionScript)

(fn StartRound
  (bind _outactors (Actor|GetAllActorsOfClass "/Game/Blueprints/BP_EnemySpawnPoint.BP_EnemySpawnPoint_C"))
  (Game|SpawnActorfromClass "/Game/Blueprints/BP_Enemy.BP_Enemy_C" (Transformation|GetActorTransform (.OutItem (Utilities|Array|Random _outactors))) "Undefined" 0 0))