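; BP_Sword_Player is a sword, apparently the player's, meant to destroy enemies on contact.
; When its capsule overlaps an actor tagged Enemy, it casts that same overlapped actor to BP_Player and destroys it if Swordused is true.
; Actors that fail that cast are left untouched.
; The Hit event is empty, and alternative destroy logic with debug prints sits disconnected.
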(event OnComponentBeginOverlap(Capsule)
  (params (OverlappedComponent :type Primitive%20Component%20Object%20Reference) (OtherActor :type Actor%20Object%20Reference) (OtherComp :type Primitive%20Component%20Object%20Reference) (OtherBodyIndex :type Integer) (bFromSweep :type Boolean) (SweepResult :type Hit%20Result%20Structure%20%28by%20ref%29))
  (if (Actor|ActorHasTag OtherActor "Enemy")
    (bind _asbp_player (Utilities|Casting|CastToBP_Player OtherActor))
    (if (Variables|/Game/Blueprints/BP_Player.BP_Player_C|GetSwordused _asbp_player)
      (Actor|DestroyActor OtherActor))))

(event Collision|EventHit
  (params (MyComp :type Primitive%20Component%20Object%20Reference) (Other :type Actor%20Object%20Reference) (OtherComp :type Primitive%20Component%20Object%20Reference) (bSelfMoved :type Boolean) (HitLocation :type Vector :default "0, 0, 0") (HitNormal :type Vector :default "0, 0, 0") (NormalImpulse :type Vector :default "0, 0, 0") (Hit :type Hit%20Result%20Structure%20%28by%20ref%29)))

(fn ConstructionScript)